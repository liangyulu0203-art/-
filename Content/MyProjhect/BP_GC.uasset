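; BP_GC is a game controller Blueprint that creates the game UI and drives a shooting-direction actor.
; BeginPlay adds WBP_GmUI to the viewport and caches the BP_方向 direction actor found in the level.
; The ONBPCLICK event plays a timeline that lerps the shooting angle across a half circle and applies it as that actor's yaw.
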(event Custom|ONBPCLICK
  (Development|PrintString "開始事件")
  (bind _newtrack_0 (Timeline|Timeline Play)
    (:Update
      (bind _output_get (Variables|Default|Set射擊角度 (Math|Float|Lerp 1.8e+02 0.0 _newtrack_0)))
      (Transformation|SetActorRotation (Variables|Default|Get方向變數) (Math|Rotator|MakeRotator 0.0 0.0 _output_get)))))

(event EventBeginPlay
  (Development|PrintString "GameController 開始載入")
  ;[0.15 0.15 0.15 0.5] 設立UI
  (bind _returnvalue (UserInterface|CreateWidget "/Game/MyProjhect/WBP_GmUI.WBP_GmUI_C"))
  (UserInterface|Viewport|AddtoViewport _returnvalue 0)
  ;[0.15 0.15 0.15 0.5] 取得方向
  (bind _returnvalue_2 (Actor|GetActorOfClass "/Game/MyProjhect/BP_方向.BP_方向_C"))
  (Variables|Default|Set方向變數 _returnvalue_2))

(event EventTick
  (params (DeltaSeconds :type Float%20%28single-precision%29)))

(fn ConstructionScript)